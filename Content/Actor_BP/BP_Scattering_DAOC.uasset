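; BP_Scattering_DAOC is a scattering actor that places randomized static mesh instances across a rectangular region, built entirely in the construction script.
; It creates one instanced mesh component per entry in the Mesh array.
; Seeded random points get vertical Visibility traces, and the hit location is used without a hit check.
; The same stream sets rotation (yaw-only or all axes), optional per-axis scale and the mesh for each instance.
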(event EventBeginPlay)

(event Collision|EventActorBeginOverlap
  (params (OtherActor :type Actor%20Object%20Reference)))

(event EventTick
  (params (DeltaSeconds :type Float%20%28single-precision%29)))

(fn ConstructionScript
  (bind _mesh (Variables|Default|GetMesh))
  (bind _collision_region (Variables|Default|GetCollision%20Region))
  (bind _random_position (Variables|Default|GetRandom%20Position))
  (bind _instanced_mesh_bank (Variables|Default|GetInstanced%20Mesh%20Bank))
  (bind _random_position_2 (Variables|Default|GetRandom%20Position))
  (bind _random_position_3 (Variables|Default|GetRandom%20Position))
  (bind _max_random_rotation (Variables|Rotation|GetMax%20Random%20Rotation))
  (bind _max_random_scale (Variables|Scale|GetMax%20Random%20scale))
  (bind _minimum_random_scale (Variables|Scale|GetMinimum%20Random%20Scale))
  (bind _returnvalue (Math|Random|RandomFloatinRangefromStream _minimum_random_scale _max_random_scale _random_position))
  (Utilities|FlowControl|Sequence
    (:then_0
      ;[1 1 1] Set Static Mesh
      (for _index (range 0 (Utilities|Array|LastIndex _mesh))
        (bind _returnvalue_2 (AddComponent|AddInstancedStaticMeshComponent false))
        (Components|StaticMesh|SetStaticMesh _returnvalue_2 (Utilities|Array|Get(acopy) _mesh _index))
        (Utilities|Array|Add (Variables|Default|GetInstanced%20Mesh%20Bank) _returnvalue_2)))
    (:then_1
      ;[1 1 1] Position
      (for _index_2 (range 0 (Variables|Default|GetInstances%20to%20Spawn))
        (Variables|Default|SetSpawn%20Point (Math|Vector|MakeVector (Math|Random|RandomFloatinRangefromStream 0.0 (Variables|Default|GetRegion%20X) (Variables|Default|GetRandom%20Position)) (Math|Random|RandomFloatinRangefromStream 0.0 (Variables|Default|GetRegion%20Y) (Variables|Default|GetRandom%20Position)) 0.0))
        (bind _outhit (Collision|LineTraceByChannel (+ (+ (Transformation|GetActorLocation) (Variables|Default|GetSpawn%20Point)) (Math|Vector|MakeVector 0.0 0.0 _collision_region)) (- (+ (Transformation|GetActorLocation) (Variables|Default|GetSpawn%20Point)) (Math|Vector|MakeVector 0.0 0.0 _collision_region)) "TraceTypeQuery1" false 0 "ForOneFrame"))
        ;[1 1 1] Rotation
        (if (Variables|Rotation|GetRotate%20All%20Axis)
          (if (Variables|Rotation|GetRotate%20All%20Axis%20Auto)
            (Variables|Rotation|SetRotation (Math|Rotator|MakeRotator (Math|Random|RandomFloatinRangefromStream 0.0 3.6e+02 _random_position_2) (Math|Random|RandomFloatinRangefromStream 0.0 3.6e+02 _random_position_2) (Math|Random|RandomFloatinRangefromStream 0.0 3.6e+02 _random_position_2)))
            (else
              (Variables|Rotation|SetRotation (Math|Rotator|MakeRotator (Math|Random|RandomFloatinRangefromStream 0.0 _max_random_rotation _random_position_3) (Math|Random|RandomFloatinRangefromStream 0.0 _max_random_rotation _random_position_3) (Math|Random|RandomFloatinRangefromStream 0.0 _max_random_rotation _random_position_3)))))
          (else
            (Variables|Rotation|SetRotation (Math|Rotator|MakeRotator 0.0 0.0 (Math|Random|RandomFloatinRangefromStream 0.0 3.6e+02 _random_position_2)))))
        ;[1 1 1] Scale
        (if (Variables|Scale|GetRandom%20Scale)
          (Variables|Default|SetScale (Math|Vector|MakeVector _returnvalue _returnvalue _returnvalue))
          (else
            (Variables|Default|SetScale (.scale (Transformation|GetRelativeTransform _returnvalue_2)))))
        ;[1 1 1] Add Instance
        (Components|InstancedStaticMesh|AddInstance (Utilities|Array|Get(acopy) _instanced_mesh_bank (Math|Random|RandomIntegerinRangefromStream 0 (Utilities|Array|LastIndex _instanced_mesh_bank) (Variables|Default|GetRandom%20Position))) (Math|Transform|MakeTransform (- (.Location (Collision|BreakHitResult _outhit)) (.location (Transformation|GetActorTransform))) (Variables|Rotation|GetRotation) (Variables|Default|GetScale)))))))