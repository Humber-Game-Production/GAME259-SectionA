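; BP_Ladder_PEN is a climbable ladder actor with configurable height, built procedurally in its construction script.
; The construction script stacks mesh segments from the mesh bounds and target height, then sizes and positions a climb trigger box and a collision box to fit.
; Overlapping the climb volume enables climbing on BP_Character_PEN and passes it the climb speed and ladder up vector; leaving disables climbing.
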(event OnComponentBeginOverlap(ClimbVolume)
  (params (OverlappedComponent :type Primitive%20Component%20Object%20Reference) (OtherActor :type Actor%20Object%20Reference) (OtherComp :type Primitive%20Component%20Object%20Reference) (OtherBodyIndex :type Integer) (bFromSweep :type Boolean) (SweepResult :type Hit%20Result%20Structure%20%28by%20ref%29))
  (bind _asbp_character_pen (Utilities|Casting|CastToBP_Character_PEN OtherActor))
  (Variables|/Game/Game_BP/Character/BP_Character_PEN.BP_Character_PEN_C|SetCanClimbLadder _asbp_character_pen true)
  (Variables|/Game/Game_BP/Character/BP_Character_PEN.BP_Character_PEN_C|SetClimbSpeed _asbp_character_pen (Variables|Default|GetLadderClimbSpeed))
  (Variables|/Game/Game_BP/Character/BP_Character_PEN.BP_Character_PEN_C|SetClimbDirectionVector _asbp_character_pen (Math|Vector|GetUpVector (Transformation|GetActorRotation))))

(event OnComponentEndOverlap(ClimbVolume)
  (params (OverlappedComponent :type Primitive%20Component%20Object%20Reference) (OtherActor :type Actor%20Object%20Reference) (OtherComp :type Primitive%20Component%20Object%20Reference) (OtherBodyIndex :type Integer))
  (bind _asbp_character_pen (Utilities|Casting|CastToBP_Character_PEN OtherActor))
  (Variables|/Game/Game_BP/Character/BP_Character_PEN.BP_Character_PEN_C|SetCanClimbLadder _asbp_character_pen false))

(fn ConstructionScript
  (bind _climbvolume (Variables|Default|GetClimbVolume))
  (bind _laddercollision (Variables|Default|GetLadderCollision))
  (bind _laddermesh (Variables|Default|GetLadderMesh))
  (bind _returnvalue (StaticMesh|GetBounds _laddermesh))
  (Utilities|FlowControl|Sequence
    (:then_0
      ;[1 1 1] Variables
      (LocalVariables|SetLadderBounds (+ (.origin _returnvalue) (.boxextent _returnvalue)))
      (Variables|/Script/Engine.PrimitiveComponent|SetbGenerateOverlapEvents (Variables|Default|GetClimbVolume) (Variables|Default|GetAllow%20Climbing)))
    (:then_1
      ;[1 1 1] Ladder
      (LocalVariables|SetNumLadderSegments (Math|Float|Truncate (/ (Variables|Default|GetLadderHeight) (.z (LocalVariables|GetLadderBounds)))))
      (for _index (range 0 (Math|Float|Truncate (/ (Variables|Default|GetLadderHeight) (.z (LocalVariables|GetLadderBounds)))))
        (bind _returnvalue_2 (AddComponent|AddStaticMeshComponent false))
        (Components|StaticMesh|SetStaticMesh _returnvalue_2 (Variables|Default|GetLadderMesh))
        (Transformation|SetRelativeLocation _returnvalue_2 (Math|Vector|MakeVector 0.0 0.0 (* _index (.z (LocalVariables|GetLadderBounds)))) false false)))
    (:then_2
      ;[1 1 1] ClimbVolume
      (Components|Box|SetBoxExtent _climbvolume (Math|Vector|MakeVector 2.0 2.0 (/ (* (+ (LocalVariables|GetNumLadderSegments) 1) (.z (LocalVariables|GetLadderBounds))) 2.0)) true)
      (Transformation|SetRelativeLocation _climbvolume (Math|Vector|MakeVector 0.0 (* (.x (LocalVariables|GetLadderBounds)) (Variables|Default|GetCollision%20Distance)) (/ (* (+ (LocalVariables|GetNumLadderSegments) 1) (.z (LocalVariables|GetLadderBounds))) 2.0)) false false))
    (:then_3
      ;[1 1 1] ClimbVolume
      (Components|Box|SetBoxExtent _laddercollision (Math|Vector|MakeVector (.x (LocalVariables|GetLadderBounds)) (.y (LocalVariables|GetLadderBounds)) (/ (+ (* (+ (LocalVariables|GetNumLadderSegments) 1) (.z (LocalVariables|GetLadderBounds))) (Variables|Default|GetCollisionTopOffset)) 2.0)) true)
      (Transformation|SetRelativeLocation _laddercollision (Math|Vector|MakeVector 0.0 0.0 (/ (+ (* (+ (LocalVariables|GetNumLadderSegments) 1) (.z (LocalVariables|GetLadderBounds))) (Variables|Default|GetCollisionTopOffset)) 2.0)) false false))))