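; BP_Amulet_DORH is an amulet actor whose material changes colour and flickers when the ThirdPersonCharacter enters its AmuletBox trigger.
; BeginPlay creates a dynamic material instance on the static mesh; the ColourFade timeline drives its Color and EColor on overlap and reverses on exit.
; Each ColourFade update also calls Play on the Emmission_Flicker timeline, which drives Emissive and is never explicitly stopped.
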(event OnComponentBeginOverlap(AmuletBox)
  (params (OverlappedComponent :type Primitive%20Component%20Object%20Reference) (OtherActor :type Actor%20Object%20Reference) (OtherComp :type Primitive%20Component%20Object%20Reference) (OtherBodyIndex :type Integer) (bFromSweep :type Boolean) (SweepResult :type Hit%20Result%20Structure%20%28by%20ref%29))
  (Utilities|Casting|CastToThirdPersonCharacter OtherActor)
  (bind _colourfade (Timeline|ColourFade Play)
    (:Update
      (Rendering|Material|SetVectorParameterValue (stale EventBeginPlay _returnvalue) "Color" _colourfade :!class /Script/Engine.MaterialInstanceDynamic)
      (Rendering|Material|SetVectorParameterValue (stale EventBeginPlay _returnvalue) "EColor" _colourfade :!class /Script/Engine.MaterialInstanceDynamic)
      (bind _emmission (Timeline|Emmission_Flicker Play)
        (:Update
          (Rendering|Material|SetScalarParameterValue (stale EventBeginPlay _returnvalue) "Emissive" _emmission :!class /Script/Engine.MaterialInstanceDynamic))))))

(event OnComponentEndOverlap(AmuletBox)
  (params (OverlappedComponent :type Primitive%20Component%20Object%20Reference) (OtherActor :type Actor%20Object%20Reference) (OtherComp :type Primitive%20Component%20Object%20Reference) (OtherBodyIndex :type Integer))
  (Utilities|Casting|CastToThirdPersonCharacter OtherActor)
  (bind _colourfade (Timeline|ColourFade Reverse)
    (:Update
      (Rendering|Material|SetVectorParameterValue (stale EventBeginPlay _returnvalue) "Color" _colourfade :!class /Script/Engine.MaterialInstanceDynamic)
      (Rendering|Material|SetVectorParameterValue (stale EventBeginPlay _returnvalue) "EColor" _colourfade :!class /Script/Engine.MaterialInstanceDynamic)
      (bind _emmission (Timeline|Emmission_Flicker Play)
        (:Update
          (Rendering|Material|SetScalarParameterValue (stale EventBeginPlay _returnvalue) "Emissive" _emmission :!class /Script/Engine.MaterialInstanceDynamic))))))

(event EventBeginPlay
  (bind _returnvalue (Rendering|Material|CreateDynamicMaterialInstance (Variables|Default|GetStaticMesh) 0 "/Game/Assets/Materials/M_DynamicMaterial_DAOC.M_DynamicMaterial_DAOC" "None" :!class /Script/Engine.PrimitiveComponent)))

(fn ConstructionScript)