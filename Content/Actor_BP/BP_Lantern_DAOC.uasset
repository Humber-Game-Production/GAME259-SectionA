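; BP_Lantern_DAOC is a lantern actor that provides a flickering light.
; The construction script applies its intensity, color and radius variables to the LanternLight component.
; On BeginPlay, the LightFlicker timeline starts and multiplies its curve value by the base intensity to drive the light's brightness on each update.
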(event EventBeginPlay
  (bind _intensity (Timeline|LightFlicker Play)
    (:Update
      (Rendering|Components|Light|SetIntensity (Variables|Default|GetLanternLight) (* _intensity (Variables|Default|GetIntensity))))))

(fn ConstructionScript
  (bind _lanternlight (Variables|Default|GetLanternLight))
  (Rendering|Components|Light|SetIntensity _lanternlight (Variables|Default|GetIntensity))
  (Rendering|Components|Light|SetLightColor _lanternlight (Math|Conversions|ToLinearColor(Color) (Variables|Default|GetColor)) true)
  (Rendering|Lighting|SetAttenuationRadius _lanternlight (Variables|Default|GetLightRadius)))