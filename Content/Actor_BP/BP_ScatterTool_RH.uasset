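; BP_ScatterTool_RH is an editor scatter tool that randomly places instanced static meshes across a rectangular region extending from the actor's location.
; Its construction script creates one instanced static mesh component per entry in the Mesh array.
; It then line-traces vertically at seeded random points and adds a randomly chosen mesh's instance at each hit.
; Separate random streams drive position and mesh choice, while rotation and scale are not randomized.
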(event EventBeginPlay)

(event Collision|EventActorBeginOverlap
  (params (OtherActor :type Actor%20Object%20Reference)))

(event EventTick
  (params (DeltaSeconds :type Float%20%28single-precision%29)))

(fn ConstructionScript
  (bind _mesh (Variables|Default|GetMesh))
  (bind _instanced_mesh_component_bank (Variables|Default|GetInstanced%20Mesh%20Component%20Bank))
  (bind _collision_region (Variables|Default|GetCollision%20Region))
  (Utilities|FlowControl|Sequence
    (:then_0
      ;[1 1 1] Set Mesh
      (for _index (range 0 (Utilities|Array|LastIndex _mesh))
        (bind _returnvalue (AddComponent|AddInstancedStaticMeshComponent false))
        (Components|StaticMesh|SetStaticMesh _returnvalue (Utilities|Array|Get(acopy) _mesh _index))
        (Utilities|Array|Add (Variables|Default|GetInstanced%20Mesh%20Component%20Bank) _returnvalue)))
    (:then_1
      (for _index_2 (range 0 (Variables|Default|GetInstances%20of%20Spawn))
        (Variables|Default|SetSpawn%20Point (Math|Vector|MakeVector (Math|Random|RandomFloatinRangefromStream 0.0 (Variables|Default|GetRegion%20X) (Variables|Default|GetRandom%20Position)) (Math|Random|RandomFloatinRangefromStream 0.0 (Variables|Default|GetRegion%20Y) (Variables|Default|GetRandom%20Position)) 0.0))
        (bind (_outhit _returnvalue_2) (Collision|LineTraceByChannel (+ (+ (Transformation|GetActorLocation) (Variables|Default|GetSpawn%20Point)) (Math|Vector|MakeVector 0.0 0.0 _collision_region)) (- (+ (Transformation|GetActorLocation) (Variables|Default|GetSpawn%20Point)) (Math|Vector|MakeVector 0.0 0.0 _collision_region)) "TraceTypeQuery1" false 0 "ForOneFrame"))
        (if _returnvalue_2
          ;[1 1 1] Spawning Mesh
          (Components|InstancedStaticMesh|AddInstance (Utilities|Array|Get(acopy) _instanced_mesh_component_bank (Math|Random|RandomIntegerinRangefromStream 0 (Utilities|Array|LastIndex _instanced_mesh_component_bank) (Variables|Default|GetStream))) (Math|Transform|MakeTransform (- (.Location (Collision|BreakHitResult _outhit)) (Transformation|GetActorLocation)) (.rotation (Transformation|GetRelativeTransform _returnvalue)) (.scale (Transformation|GetRelativeTransform _returnvalue)))))))))