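; Construction-time generator actor that places copies of a chosen static mesh along the RoadTrack spline.
; The construction script adds an instanced static mesh component, then creates a set number of instances at even spacing along the spline.
; Each instance takes the spline's local location and rotation at that distance, plus per-axis rotation offsets.
; The event graph holds no active logic.
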(event EventBeginPlay)

(event Collision|EventActorBeginOverlap
  (params (OtherActor :type Actor%20Object%20Reference)))

(event EventTick
  (params (DeltaSeconds :type Float%20%28single-precision%29)))

(fn ConstructionScript
  (bind _roadtrack (Variables|Default|GetRoadTrack))
  (bind _returnvalue (AddComponent|AddInstancedStaticMeshComponent false))
  (Components|StaticMesh|SetStaticMesh _returnvalue (Variables|Default|GetStatic%20Mesh))
  (for _index (range 0 (- (Variables|Default|GetInstances) 1))
    (Components|InstancedStaticMesh|AddInstance _returnvalue (Math|Transform|MakeTransform (Spline|GetLocationatDistanceAlongSpline _roadtrack (* _index (Variables|Default|GetSpacing)) "Local") (Math|Rotator|MakeRotator (+ (.roll (Spline|GetRotationatDistanceAlongSpline _roadtrack (* _index (Variables|Default|GetSpacing)) "Local")) (Variables|Default|GetRotation_Offset_X)) (+ (.pitch (Spline|GetRotationatDistanceAlongSpline _roadtrack (* _index (Variables|Default|GetSpacing)) "Local")) (Variables|Default|GetRotation_Offset_Y)) (+ (.yaw (Spline|GetRotationatDistanceAlongSpline _roadtrack (* _index (Variables|Default|GetSpacing)) "Local")) (Variables|Default|GetRotation_Offest_Z))) "1,1,1"))))