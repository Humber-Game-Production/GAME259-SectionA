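; BP_RoadGenerator_DAOC is a road generator actor that builds a mesh road along its RoadTrack spline in the construction script.
; It adds one spline mesh component per segment between consecutive points, using the StaticMesh variable and query-and-physics collision.
; Segment ends take local-space positions at each point's distance along the spline, with direction vectors rather than spline tangents as their tangents.
; The event graph has no active logic.
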(event EventBeginPlay)

(event Collision|EventActorBeginOverlap
  (params (OtherActor :type Actor%20Object%20Reference)))

(event EventTick
  (params (DeltaSeconds :type Float%20%28single-precision%29)))

(fn ConstructionScript
  (bind _roadtrack (Variables|Default|GetRoadTrack))
  (for _index (range 0 (- (Spline|GetNumberOfSplinePoints (Variables|Default|GetRoadTrack)) 2))
    (bind _returnvalue (AddComponent|AddSplineMeshComponent false))
    (Components|StaticMesh|SetStaticMesh _returnvalue (Variables|Default|GetStatic%20Mesh))
    (SplineMesh|SetStartandEnd _returnvalue (Spline|GetLocationatDistanceAlongSpline _roadtrack (Spline|GetDistanceAlongSplineatSplinePoint _roadtrack _index) "Local") (Spline|GetDirectionatDistanceAlongSpline _roadtrack (Spline|GetDistanceAlongSplineatSplinePoint _roadtrack _index) "Local") (Spline|GetLocationatDistanceAlongSpline _roadtrack (Spline|GetDistanceAlongSplineatSplinePoint _roadtrack (+ _index 1)) "Local") (Spline|GetDirectionatDistanceAlongSpline _roadtrack (Spline|GetDistanceAlongSplineatSplinePoint _roadtrack (+ _index 1)) "Local") false :!class /Script/Engine.SplineMeshComponent)
    (Collision|SetCollisionEnabled _returnvalue "QueryAndPhysics")))