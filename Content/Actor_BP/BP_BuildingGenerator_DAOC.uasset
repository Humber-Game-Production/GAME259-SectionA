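; Procedural building actor that stacks modular wall meshes to a configurable floor count and caps them with a roof mesh.
; The construction script builds front, left and right walls (no back), using mesh bounds for spacing and placing the roof from the front-wall loop's index.
; Each wall piece gets its own single-instance Instanced Static Mesh component and a dynamic material tinted by Color.
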(event EventBeginPlay)

(event Collision|EventActorBeginOverlap
  (params (OtherActor :type Actor%20Object%20Reference)))

(event EventTick
  (params (DeltaSeconds :type Float%20%28single-precision%29)))

(fn ConstructionScript
  (bind _bodymesh (Variables|Default|GetBodyMesh))
  (bind _bodymesh_2 (Variables|Default|GetBodyMesh))
  (bind _returnvalue (StaticMesh|GetBoundingBox _bodymesh_2))
  (bind _returnvalue_2 (StaticMesh|GetBoundingBox _bodymesh))
  (bind _max (Utilities|Struct|BreakBox _returnvalue))
  (bind (_min _max_2) (Utilities|Struct|BreakBox _returnvalue_2))
  (Utilities|FlowControl|Sequence
    (:then_0
      ;[1 1 1] FrontWall
      (for _index (range 0 (- (Variables|Default|GetFloors) 1))
        (bind _returnvalue_3 (AddComponent|AddInstancedStaticMeshComponent false))
        (Components|StaticMesh|SetStaticMesh _returnvalue_3 (Variables|Default|GetBodyMesh))
        (Components|InstancedStaticMesh|AddInstance _returnvalue_3 (Math|Transform|MakeTransform (Math|Vector|MakeVector 0.0 0.0 (* _index (.z (.Max (Utilities|Struct|BreakBox (StaticMesh|GetBoundingBox (Variables|Default|GetBodyMesh)))))))))
        (bind _returnvalue_4 (Rendering|Material|CreateDynamicMaterialInstance _returnvalue_3 0 "/Game/Assets/MaterialInstances/Rock/BG_Buildings/MI_BGRock2_s_DAOC.MI_BGRock2_s_DAOC" "Colour" :!class /Script/Engine.PrimitiveComponent))
        (Rendering|Material|SetVectorParameterValue _returnvalue_4 "Colour" (Variables|Default|GetColor) :!class /Script/Engine.MaterialInstanceDynamic)))
    (:then_1
      ;[1 1 1] Roof
      (bind _returnvalue_5 (AddComponent|AddInstancedStaticMeshComponent false))
      (Components|StaticMesh|SetStaticMesh _returnvalue_5 (Variables|Default|GetRoof%20Mesh))
      (Components|InstancedStaticMesh|AddInstance _returnvalue_5 (Math|Transform|MakeTransform (Math|Vector|MakeVector 0.0 0.0 (* _index (.z (.Max (Utilities|Struct|BreakBox (StaticMesh|GetBoundingBox (Variables|Default|GetBodyMesh))))))))))
    (:then_2
      ;[1 1 1] LeftWall
      (for _index_2 (range 0 (- (Variables|Default|GetFloors) 1))
        (bind _returnvalue_6 (AddComponent|AddInstancedStaticMeshComponent false))
        (Components|StaticMesh|SetStaticMesh _returnvalue_6 (Variables|Default|GetBodyMesh))
        (Components|InstancedStaticMesh|AddInstance _returnvalue_6 (Math|Transform|MakeTransform (Math|Vector|MakeVector (/ (.x (.max (StaticMesh|GetBoundingBox (Variables|Default|GetRoof%20Mesh)))) 2.0) (.y _min) (* _index_2 (.z _max_2))) "0,90.000000, 0"))
        (bind _returnvalue_7 (Rendering|Material|CreateDynamicMaterialInstance _returnvalue_6 0 "/Game/Assets/MaterialInstances/Rock/BG_Buildings/MI_BGRock2_s_DAOC.MI_BGRock2_s_DAOC" "Colour" :!class /Script/Engine.PrimitiveComponent))
        (Rendering|Material|SetVectorParameterValue _returnvalue_7 "Colour" (Variables|Default|GetColor) :!class /Script/Engine.MaterialInstanceDynamic)))
    (:then_3
      ;[1 1 1] RightWall
      (for _index_3 (range 0 (- (Variables|Default|GetFloors) 1))
        (bind _returnvalue_8 (AddComponent|AddInstancedStaticMeshComponent false))
        (Components|StaticMesh|SetStaticMesh _returnvalue_8 (Variables|Default|GetBodyMesh))
        (Components|InstancedStaticMesh|AddInstance _returnvalue_8 (Math|Transform|MakeTransform (Math|Vector|MakeVector (/ (.x (.max (StaticMesh|GetBoundingBox (Variables|Default|GetRoof%20Mesh)))) 2.0) (.y _max) (* _index_3 (.z _max))) "0,270.000000, 0"))
        (bind _returnvalue_9 (Rendering|Material|CreateDynamicMaterialInstance _returnvalue_8 0 "/Game/Assets/MaterialInstances/Rock/BG_Buildings/MI_BGRock2_s_DAOC.MI_BGRock2_s_DAOC" "Colour" :!class /Script/Engine.PrimitiveComponent))
        (Rendering|Material|SetVectorParameterValue _returnvalue_9 "Colour" (Variables|Default|GetColor) :!class /Script/Engine.MaterialInstanceDynamic)))))