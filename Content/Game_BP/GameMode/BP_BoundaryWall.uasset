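; BP_BoundaryWall is a timed barrier for CTF rounds that blocks for a set Duration, then opens.
; On BeginPlay it binds Block to the CTFGameState round start delegate and starts the countdown.
; Block shows the Plane, enables collision and tick, then re-enters the same Delay.
; When the Delay ends, the wall hides the Plane and turns off collision and tick.
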(event Custom|Block
  (Development|SetHiddeninGame (Variables|Default|GetPlane) false false)
  (Collision|SetActorEnableCollision true)
  (Actor|Tick|SetActorTickEnabled true)
  (Utilities|FlowControl|Delay (Variables|Default|GetDuration))
  (Development|SetHiddeninGame (Variables|Default|GetPlane) true false)
  (Collision|SetActorEnableCollision false)
  (Actor|Tick|SetActorTickEnabled false))

(event EventBeginPlay
  (bind _asctfgame_state (Utilities|Casting|CastToCTFGameState (Game|GetGameState)))
  (EventDispatchers|BindEventtoRoundStartDelegate _asctfgame_state (delegate Custom|Block))
  (Utilities|FlowControl|Delay (Variables|Default|GetDuration))
  (Development|SetHiddeninGame (Variables|Default|GetPlane) true false)
  (Collision|SetActorEnableCollision false)
  (Actor|Tick|SetActorTickEnabled false))

(fn ConstructionScript)