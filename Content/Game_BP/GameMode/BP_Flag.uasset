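; BP_Flag is a capture-the-flag objective, called an amulet in its debug prints, that recolors by team and can be dropped.
; A timeline started on BeginPlay animates emissive glow on a dynamic material, whose colors change when an overlapping pawn's player state reports Human or Alien.
; Drop, also bound to key 1, disables input, detaches, and line-traces down to rest above the ground, returning to its initial location on a miss.
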(event Collision|EventActorBeginOverlap
  (params (OtherActor :type Actor%20Object%20Reference))
  (bind _aspawn (Utilities|Casting|CastToPawn OtherActor))
  (bind _asctfplayer_state (Utilities|Casting|CastToCTFPlayerState (Variables|/Script/Engine.Pawn|GetPlayerState _aspawn)))
  (switch Utilities|FlowControl|Switch|SwitchonETeamIdentifier (Variables|/Script/GAME259A.CTFPlayerState|GetteamID _asctfplayer_state)
    (:Human
      (Rendering|Material|SetVectorParameterValue (stale EventBeginPlay _returnvalue) "Color" "(R=0.973958,G=0.021794,B=0.000000,A=1.000000)" :!class /Script/Engine.MaterialInstanceDynamic)
      (Rendering|Material|SetVectorParameterValue (stale EventBeginPlay _returnvalue) "Ecolor" "(R=0.989583,G=0.000000,B=0.057201,A=1.000000)" :!class /Script/Engine.MaterialInstanceDynamic)
      (Development|PrintString "Human touched Amulet"))
    (:Alien
      (Rendering|Material|SetVectorParameterValue (stale EventBeginPlay _returnvalue) "Color" "(R=0.070961,G=0.561157,B=0.973958,A=1.000000)" :!class /Script/Engine.MaterialInstanceDynamic)
      (Rendering|Material|SetVectorParameterValue (stale EventBeginPlay _returnvalue) "Ecolor" "(R=0.076278,G=0.677836,B=0.989583,A=1.000000)" :!class /Script/Engine.MaterialInstanceDynamic)
      (Development|PrintString "Alien touched Amulet"))))

(event EventBeginPlay
  (bind _returnvalue (Rendering|Material|CreateDynamicMaterialInstance (Variables|Character|GetMesh) 0 "/Game/Assets/Materials/M_DynamicMaterial_DAOC.M_DynamicMaterial_DAOC" "None" :!class /Script/Engine.PrimitiveComponent))
  (bind _emmission (Timeline|Timeline_0 Play)
    (:Update
      (Rendering|Material|SetScalarParameterValue _returnvalue "Emissive" _emmission :!class /Script/Engine.MaterialInstanceDynamic))))

(event EventDrop
  (bind _returnvalue (Transformation|GetActorLocation))
  ;[1 1 1] Drop Flag
  (Development|PrintString "Drop Flag")
  (Input|DisableInput 0)
  (Transformation|DetachFromActor "KeepWorld" "KeepRelative" "KeepRelative")
  (bind _outhit (Collision|LineTraceByChannel _returnvalue (- _returnvalue "0, 0,2500.000000") "TraceTypeQuery1" false 0 "ForDuration"))
  (if (.bBlockingHit (Collision|BreakHitResult _outhit))
    (Transformation|SetActorLocation (+ (.Location (Collision|BreakHitResult _outhit)) (Variables|Default|GetDistanceFromGround)) false false)
    (else
      (Transformation|SetActorLocation (Variables|Default|GetInitLocation) false false))))

(event Input|KeyboardEvents|1
  (params (Key :type Key%20Structure :default "None"))
  (bind _returnvalue (Transformation|GetActorLocation))
  ;[1 1 1] Drop Flag
  (:Pressed
    (Development|PrintString "Pressed 1 in BP_Flag")
    (Development|PrintString "Drop Flag")
    (Input|DisableInput 0)
    (Transformation|DetachFromActor "KeepWorld" "KeepRelative" "KeepRelative")
    (bind _outhit (Collision|LineTraceByChannel _returnvalue (- _returnvalue "0, 0,2500.000000") "TraceTypeQuery1" false 0 "ForDuration"))
    (if (.bBlockingHit (Collision|BreakHitResult _outhit))
      (Transformation|SetActorLocation (+ (.Location (Collision|BreakHitResult _outhit)) (Variables|Default|GetDistanceFromGround)) false false)
      (else
        (Transformation|SetActorLocation (Variables|Default|GetInitLocation) false false)))))

(fn ConstructionScript)