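; Throwable combat rock projectile that damages enemy-team characters in capture-the-flag play.
; BeginProjectile adds projectile movement at launch; on hit it starts a despawn timer, checks CTF team IDs, damages enemies once and attaches to the struck bone.
; While aiming, Tick predicts the charged-throw path, rebuilding spline meshes along it each frame and placing a HitPoint marker whose material changes after an overlap.
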(event OnComponentHit(Sphere)
  (params (HitComponent :type Primitive%20Component%20Object%20Reference) (OtherActor :type Actor%20Object%20Reference) (OtherComp :type Primitive%20Component%20Object%20Reference) (NormalImpulse :type Vector :default "0, 0, 0") (Hit :type Hit%20Result%20Structure%20%28by%20ref%29))
  (bind _sphere (Variables|Default|GetSphere))
  (if (Variables|Default|GetIsFired)
    (Transformation|SetActorLocation self (+ (* (Math|Vector|GetForwardVector _sphere) 1e+02) (Transformation|GetWorldLocation _sphere)) false false)
    (Actor|SetLifeSpan 5.0)
    (bind _asbase_character_bp (Utilities|Casting|CastToBaseCharacter_BP OtherActor))
    (if (not (Variables|/Game/Game_BP/Character/BaseCharacter_BP.BaseCharacter_BP_C|GetIsAlreadyHit _asbase_character_bp))
      (bind _asbase_character_bp_2 (Utilities|Casting|CastToBaseCharacter_BP (Components|GetOwner)))
      (bind _asctfplayer_state (Utilities|Casting|CastToCTFPlayerState (Variables|/Script/Engine.Pawn|GetPlayerState _asbase_character_bp)))
      (bind _asctfplayer_state_2 (Utilities|Casting|CastToCTFPlayerState (Variables|/Script/Engine.Pawn|GetPlayerState _asbase_character_bp_2)))
      (if (Utilities|Enum|NotEqual(Enum) (Variables|/Script/GAME259A.CTFPlayerState|GetteamID _asctfplayer_state_2) (Variables|/Script/GAME259A.CTFPlayerState|GetteamID _asctfplayer_state))
        (Development|PrintString "Non-Friendly Bow Fire")
        (if (Variables|Default|GetIsLanded)
          _
          (else
            (Game|Damage|ApplyDamage OtherActor 6e+01 (Pawn|GetController _asbase_character_bp_2) (Components|GetOwner))))
        (Transformation|AttachActorToActor OtherActor (.HitBoneName (Collision|BreakHitResult Hit)) "KeepWorld" "KeepWorld" "KeepWorld" false)
        (Variables|Default|SetIsLanded true)
        (Collision|SetActorEnableCollision false)
        (else
          (Development|PrintString "Friendly Bow Fire")
          (Variables|/Game/Game_BP/Character/BaseCharacter_BP.BaseCharacter_BP_C|SetIsAlreadyHit _asbase_character_bp false))))))

(event OnComponentBeginOverlap(HitPoint)
  (params (OverlappedComponent :type Primitive%20Component%20Object%20Reference) (OtherActor :type Actor%20Object%20Reference) (OtherComp :type Primitive%20Component%20Object%20Reference) (OtherBodyIndex :type Integer) (bFromSweep :type Boolean) (SweepResult :type Hit%20Result%20Structure%20%28by%20ref%29))
  (Utilities|Casting|CastToBaseCharacter_BP OtherActor
    (:then
      (Variables|Default|SetHitting? true))
    (:CastFailed
      (Variables|Default|SetHitting? true))))

(event Custom|BeginProjectile
  (params (initSpeed :type Float%20%28single-precision%29))
  (Variables|Default|SetIsFired true)
  (Collision|SetActorEnableCollision false)
  (bind _returnvalue (AddComponent|AddProjectileMovementComponent self))
  (bind _output_get (Variables|Default|SetProjectileComponent _returnvalue))
  (Variables|/Script/Engine.MovementComponent|SetVelocity _output_get (* (Transformation|GetActorForwardVector) (* initSpeed 2e+03)))
  (Variables|/Script/Engine.ProjectileMovementComponent|SetbRotationFollowsVelocity _output_get true)
  (Collision|SetActorEnableCollision true))

(event Custom|AddSpline
  (bind _returnvalue (AddComponent|AddSplineComponent false))
  (Variables|Default|SetPrediction%20Spline _returnvalue)
  (bind _returnvalue_2 (Game|SpawnActorfromClass "/Script/GAME259A.SplineEndPointActor" (Math|Transform|MakeTransform "0, 0, 0" "0, 0, 0" "1,1,1") "Undefined" 0 0))
  (Variables|Default|SetPrediction%20End%20Point _returnvalue_2)
  (Rendering|SetVisibility (Variables|Default|GetHitPoint) false false))

(event Custom|Destroy%20Spline
  (bind _prediction_spline (Variables|Default|GetPrediction%20Spline)
    (:then
      (Components|DestroyComponent _prediction_spline)
      (Variables|Default|SetPrediction%20Spline 0)
      (CallFunction|DestroyPredictionmeshes)
      (Actor|DestroyActor (Variables|Default|GetPrediction%20End%20Point))
      (Variables|Default|SetPrediction%20End%20Point 0)
      (Rendering|SetVisibility (Variables|Default|GetHitPoint) false false))
    (:else)))

(event Custom|Destroy%20predictionmeshes
  (for _array_element (Variables|Default|GetSpline%20Meshes)
    (Components|DestroyComponent _array_element))
  (Utilities|Array|Clear (Variables|Default|GetSpline%20Meshes)))

(event EventBeginPlay
  (Collision|IgnoreActorwhenMoving (Variables|Default|GetSphere) (Components|GetOwner) true))

(event Collision|EventActorBeginOverlap
  (params (OtherActor :type Actor%20Object%20Reference)))

(event EventTick
  (params (DeltaSeconds :type Float%20%28single-precision%29))
  (bind _hitpoint (Variables|Default|GetHitPoint))
  (bind _hitpoint_2 (Variables|Default|GetHitPoint))
  (if (Variables|Default|GetHitting?)
    (Rendering|Material|SetMaterial _hitpoint_2 0 "/Game/Game_BP/Weapons/HitPointMaterial_2.HitPointMaterial_2")
    (else
      (Rendering|Material|SetMaterial _hitpoint_2 0 "/Game/Game_BP/Weapons/HitPointMaterial.HitPointMaterial")))
  (if (Utilities|IsValid (Variables|Default|GetPrediction%20Spline))
    (Utilities|FlowControl|Sequence
      (:then_0
        (bind (_outhit _outpathpositions _outlasttracedestination _returnvalue) (Class|GameplayStatics|BlueprintPredictProjectilePathbyTraceChannel (Transformation|GetActorLocation) (* (Transformation|GetActorForwardVector) (* (* (Variables|Default|GetInitSpeedCharge) 1.5) 2e+03)) true 0.0 "ECC_WorldDynamic" true (Utilities|Array|MakeArray self 0) "None" 0.02 3e+01 1.0))
        (if _returnvalue
          (Rendering|SetVisibility _hitpoint true false)
          (Transformation|SetWorldLocation _hitpoint (+ (.ImpactPoint (Collision|BreakHitResult _outhit)) "0,0.000000,50.000000") false true)
          (else
            (Rendering|SetVisibility _hitpoint false false)))
        (Spline|SetSplinePoints (Variables|Default|GetPrediction%20Spline) _outpathpositions "World" true)
        (CallFunction|DestroyPredictionmeshes))
      (:then_1
        (for _index (range 0 (Math|Float|Truncate (/ (Spline|GetSplineLength (Variables|Default|GetPrediction%20Spline)) 1e+02)))
          (Variables|Default|SetIndex _index)
          (bind _returnvalue_2 (AddComponent|AddSplineMeshComponent true))
          (Utilities|Array|Add (Variables|Default|GetSpline%20Meshes) _returnvalue_2)
          (SplineMesh|SetStartandEnd _returnvalue_2 (Spline|GetLocationatDistanceAlongSpline (Variables|Default|GetPrediction%20Spline) (* (Variables|Default|GetIndex) 1e+02) "World") (Math|Vector|ClampVectorSize (Spline|GetTangentatDistanceAlongSpline (Variables|Default|GetPrediction%20Spline) (* (Variables|Default|GetIndex) 1e+02) "World") 0.0 1e+02) (Spline|GetLocationatDistanceAlongSpline (Variables|Default|GetPrediction%20Spline) (* (+ (Variables|Default|GetIndex) 1) 1e+02) "World") (Math|Vector|ClampVectorSize (Spline|GetTangentatDistanceAlongSpline (Variables|Default|GetPrediction%20Spline) (* (+ (Variables|Default|GetIndex) 1) 1e+02) "World") 0.0 1e+02) true :!class /Script/Engine.SplineMeshComponent))))))

(fn ConstructionScript
  (Collision|SetActorEnableCollision false))

(fn DestroyPredictionMeshes)