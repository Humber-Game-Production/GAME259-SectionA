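; Bow arrow actor that previews its flight, launches as a projectile and damages enemy-team characters.
; While aiming, a looping timer predicts the path, draws it as debug and moves a HitPoint marker to impact.
; BeginProjectile stops the preview and adds a ProjectileMovementComponent at runtime, scaled by initial speed.
; Box hits nudge the arrow forward, set its lifespan, compare CTF team IDs, then damage and bone-attach to enemies.
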(event OnComponentHit(Box)
  (params (HitComponent :type Primitive%20Component%20Object%20Reference) (OtherActor :type Actor%20Object%20Reference) (OtherComp :type Primitive%20Component%20Object%20Reference) (NormalImpulse :type Vector :default "0, 0, 0") (Hit :type Hit%20Result%20Structure%20%28by%20ref%29))
  (bind _box (Variables|Default|GetBox))
  ;[1 1 1] Hit Handling, Also pushes the arrow forward into the object to make it look cool
  (if (Variables|Default|GetIsFired)
    (Transformation|SetActorLocation self (+ (* (Math|Vector|GetForwardVector _box) 1e+02) (Transformation|GetWorldLocation _box)) false false)
    (Actor|SetLifeSpan 5.0)
    (bind _asbase_character_bp (Utilities|Casting|CastToBaseCharacter_BP OtherActor))
    (if (not (Variables|/Game/Game_BP/Character/BaseCharacter_BP.BaseCharacter_BP_C|GetIsAlreadyHit _asbase_character_bp))
      (bind _asbase_character_bp_2 (Utilities|Casting|CastToBaseCharacter_BP (Components|GetOwner)))
      (bind _asctfplayer_state (Utilities|Casting|CastToCTFPlayerState (Variables|/Script/Engine.Pawn|GetPlayerState _asbase_character_bp)))
      (bind _asctfplayer_state_2 (Utilities|Casting|CastToCTFPlayerState (Variables|/Script/Engine.Pawn|GetPlayerState _asbase_character_bp_2)))
      (if (Utilities|Enum|NotEqual(Enum) (Variables|/Script/GAME259A.CTFPlayerState|GetteamID _asctfplayer_state_2) (Variables|/Script/GAME259A.CTFPlayerState|GetteamID _asctfplayer_state))
        (Development|PrintString "Non-Friendly Bow Fire")
        (if (Variables|Default|GetIsLanded)
          _
          (else
            (Game|Damage|ApplyDamage OtherActor 3e+01 (Pawn|GetController _asbase_character_bp_2) (Components|GetOwner))))
        (Transformation|AttachActorToActor OtherActor (.HitBoneName (Collision|BreakHitResult Hit)) "KeepWorld" "KeepWorld" "KeepWorld" false)
        (Variables|Default|SetIsLanded true)
        (Collision|SetActorEnableCollision false)
        (else
          (Development|PrintString "Friendly Bow Fire")
          (Variables|/Game/Game_BP/Character/BaseCharacter_BP.BaseCharacter_BP_C|SetIsAlreadyHit _asbase_character_bp false))))))

(event Custom|BeginProjectile
  (params (initSpeed :type Float%20%28single-precision%29))
  (bind _hitpoint (Variables|Default|GetHitPoint))
  ;[1 1 1] Adds projectile to arrow, this is once the player has released right click
  (Variables|Default|SetIsFired true)
  (Utilities|Time|ClearandInvalidateTimerbyHandle (Variables|Default|GetTimerHandle))
  (Rendering|SetVisibility _hitpoint false false)
  (Transformation|SetWorldLocation _hitpoint "0, 0, 0" false true)
  (Collision|SetActorEnableCollision false)
  (bind _returnvalue (AddComponent|AddProjectileMovementComponent self))
  (bind _output_get (Variables|Default|SetProjectileComponent _returnvalue))
  (Variables|/Script/Engine.MovementComponent|SetVelocity _output_get (+ (* (Transformation|GetActorForwardVector) (* initSpeed 2e+03)) (Transformation|GetActorForwardVector (Game|GetPlayerCameraManager 0))))
  (Variables|/Script/Engine.ProjectileMovementComponent|SetbRotationFollowsVelocity _output_get true)
  (Collision|SetActorEnableCollision true))

(event Custom|PredictPath
  (bind _hitpoint (Variables|Default|GetHitPoint))
  (bind (_outhit _outpathpositions _outlasttracedestination _returnvalue) (Class|GameplayStatics|BlueprintPredictProjectilePathbyTraceChannel (Transformation|GetActorLocation) (* (Transformation|GetActorForwardVector) (* (* (Variables|Default|GetInitSpeedCharge) 1.5) 2e+03)) true 0.0 "ECC_WorldDynamic" false 0 "ForDuration" 0.02 3e+01 1.0))
  (if _returnvalue
    (Transformation|SetWorldLocation _hitpoint (.ImpactPoint (Collision|BreakHitResult _outhit)) false true)
    (Rendering|SetVisibility _hitpoint true false)))

(event Custom|PredictPathLoop
  (bind _returnvalue (Utilities|Time|SetTimerbyEvent (delegate Custom|PredictPath) 0.02 true))
  (Variables|Default|SetTimerHandle _returnvalue))

(event EventBeginPlay
  (Collision|IgnoreActorwhenMoving (Variables|Default|GetBox) (Components|GetOwner) true))

(event Collision|EventActorBeginOverlap
  (params (OtherActor :type Actor%20Object%20Reference)))

(event EventTick
  (params (DeltaSeconds :type Float%20%28single-precision%29)))

(fn ConstructionScript
  (Collision|SetActorEnableCollision false))