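; Alien character Blueprint that equips itself with a slingshot and a kukri blade for combat.
; On BeginPlay it spawns the slingshot, its separate sling piece and the blade, attaches them to hand sockets on the mesh and hides both slingshot parts.
; It then resets its already-hit flag and runs the parent BeginPlay.
; A bound OnDestroyed handler destroys the slingshot and blade, but not the sling piece.
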(event Custom|CustomEvent
  (params (DestroyedActor :type Actor%20Object%20Reference))
  (Actor|DestroyActor (Variables|Default|GetBow))
  (Actor|DestroyActor (Variables|Default|GetMelee%20Weapon)))

(event EventBeginPlay
  (bind _returnvalue (Transformation|GetActorTransform))
  (bind _mesh (Variables|Character|GetMesh))
  (bind _returnvalue_2 (Game|SpawnActorfromClass "/Game/Game_BP/Weapons/BP_SlingShotCOMBAT.BP_SlingShotCOMBAT_C" _returnvalue "AlwaysSpawn" 0 0))
  (bind _returnvalue_3 (Game|SpawnActorfromClass "/Game/Game_BP/Weapons/BP_SlingShotSling.BP_SlingShotSling_C" _returnvalue "AlwaysSpawn" 0 0))
  (Transformation|AttachComponentToComponent _returnvalue_3 _mesh "RightHandSocketSling" "SnapToTarget" "SnapToTarget" "SnapToTarget" false)
  (bind _output_get (Variables|Default|SetSlingSpecialPiece _returnvalue_3))
  (Rendering|SetActorHiddenInGame _output_get true)
  (bind _output_get_2 (Variables|Default|SetBow _returnvalue_2))
  (Transformation|AttachComponentToComponent _output_get_2 _mesh "LeftHandSocket" "SnapToTarget" "SnapToTarget" "SnapToTarget" false)
  (Rendering|SetActorHiddenInGame (Variables|Default|GetBow) true)
  (bind _returnvalue_4 (Game|SpawnActorfromClass "/Game/Game_BP/Weapons/BP_KukriBladeCOMBAT.BP_KukriBladeCOMBAT_C" (Transformation|GetActorTransform) "AlwaysSpawn" 0 0))
  (bind _output_get_3 (Variables|Default|SetMelee%20Weapon _returnvalue_4))
  (Transformation|AttachComponentToComponent _output_get_3 (Variables|Character|GetMesh) "RightHandSocket" "SnapToTarget" "SnapToTarget" "SnapToTarget" false)
  (Game|BindEventtoOnDestroyed (delegate Custom|CustomEvent))
  (Variables|Default|SetIsAlreadyHit false)
  (|CallParentFunction))

(event Collision|EventActorBeginOverlap
  (params (OtherActor :type Actor%20Object%20Reference))
  (|CallParentFunction OtherActor) ; This node is disabled and will not be called.\nDrag off pins to build functionality.
)

(event EventTick
  (params (DeltaSeconds :type Float%20%28single-precision%29))
  (|CallParentFunction DeltaSeconds) ; This node is disabled and will not be called.\nDrag off pins to build functionality.
)

(fn ConstructionScript
  (|CallParentFunction))