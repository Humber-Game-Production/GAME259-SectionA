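; BP_Character_PEN is a player Character that handles movement, look, jump and toggled crouch input.
; When CanClimbLadder is set, forward input raises the walkable floor angle and pushes forced movement along ClimbDirectionVector scaled by ClimbSpeed, while strafing is disabled.
; Otherwise the floor angle is restored and movement follows the actor's rotation.
; A FlipFlop alternates Crouch and UnCrouch on each press.
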(event EventBeginPlay)

(event Collision|EventActorBeginOverlap
  (params (OtherActor :type Actor%20Object%20Reference)))

(event Input|ActionEvents|InputActionJump
  (params (Key :type Key%20Structure))
  (:Pressed
    (Character|Jump)))

(event Input|ActionEvents|InputActionCrouch
  (params (Key :type Key%20Structure))
  (:Pressed
    (Utilities|FlowControl|FlipFlop
      (:A
        (Character|Crouch))
      (:B
        (Character|UnCrouch)))))

(event Input|AxisEvents|InputAxisFrontBack
  (params (AxisValue :type Float%20%28single-precision%29))
  (bind _charactermovement (Variables|Character|GetCharacterMovement))
  (if (Variables|Default|GetCanClimbLadder)
    (Pawn|Components|CharacterMovement|SetWalkableFloorAngle _charactermovement 91.0)
    (Pawn|Input|AddMovementInput (Variables|Default|GetClimbDirectionVector) (* AxisValue (Variables|Default|GetClimbSpeed)) true)
    (else
      (Pawn|Components|CharacterMovement|SetWalkableFloorAngle _charactermovement 44.0)
      (Pawn|Input|AddMovementInput (Math|Vector|GetForwardVector (Transformation|GetActorRotation)) AxisValue false))))

(event Input|AxisEvents|InputAxisSideToSide
  (params (AxisValue :type Float%20%28single-precision%29))
  (if (not (Variables|Default|GetCanClimbLadder))
    (Pawn|Input|AddMovementInput (Math|Vector|GetRightVector (Transformation|GetActorRotation)) AxisValue false)))

(event Input|AxisEvents|InputAxisTurn
  (params (AxisValue :type Float%20%28single-precision%29))
  (Pawn|Input|AddControllerYawInput AxisValue))

(event Input|AxisEvents|InputAxisUpDown
  (params (AxisValue :type Float%20%28single-precision%29))
  (Pawn|Input|AddControllerPitchInput AxisValue))

(fn ConstructionScript)