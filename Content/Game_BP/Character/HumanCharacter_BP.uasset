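; Human character Blueprint that equips itself with a bow and a melee axe when play begins.
; BeginPlay spawns both weapon actors, snaps them to separate left-hand mesh sockets, hides the bow, clears the already-hit flag, then runs the parent logic.
; A bound OnDestroyed handler destroys both weapons along with the character.
; Tick and overlap events are disabled, and the construction script only calls its parent.
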(event Custom|CustomEvent
  (params (DestroyedActor :type Actor%20Object%20Reference))
  (Actor|DestroyActor (Variables|Default|GetBow))
  (Actor|DestroyActor (Variables|Default|GetMelee%20Weapon)))

(event EventBeginPlay
  (bind _returnvalue (Game|SpawnActorfromClass "/Game/Game_BP/Weapons/SM_Bow_AD.SM_Bow_AD_C" (Transformation|GetActorTransform) "Undefined" 0 0))
  (bind _output_get (Variables|Default|SetBow _returnvalue))
  (Transformation|AttachComponentToComponent _returnvalue (Variables|Character|GetMesh) "LeftHandSocketRange" "SnapToTarget" "SnapToTarget" "SnapToTarget" false)
  (Rendering|SetActorHiddenInGame (Variables|Default|GetBow) true)
  (bind _returnvalue_2 (Game|SpawnActorfromClass "/Game/Game_BP/Weapons/SM_Axe_COMBAT.SM_Axe_COMBAT_C" (Transformation|GetActorTransform) "Undefined" 0 0))
  (bind _output_get_2 (Variables|Default|SetMelee%20Weapon _returnvalue_2))
  (Transformation|AttachComponentToComponent _output_get_2 (Variables|Character|GetMesh) "LeftHandSocketMelee" "SnapToTarget" "SnapToTarget" "SnapToTarget" false)
  (Game|BindEventtoOnDestroyed (delegate Custom|CustomEvent))
  (Variables|Default|SetIsAlreadyHit false)
  (|CallParentFunction))

(event Collision|EventActorBeginOverlap
  (params (OtherActor :type Actor%20Object%20Reference))
  (|CallParentFunction OtherActor) ; This node is disabled and will not be called.\nDrag off pins to build functionality.
)

(event EventTick
  (params (DeltaSeconds :type Float%20%28single-precision%29))
  (|CallParentFunction DeltaSeconds) ; This node is disabled and will not be called.\nDrag off pins to build functionality.
)

(fn ConstructionScript
  (|CallParentFunction))