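; Base multiplayer character Blueprint for a team capture-the-flag game, handling melee and ranged combat, damage and death, aim pitch updates and the pause menu.
; Left click triggers a delayed sphere-overlap melee hit that damages only enemy players.
; Ranged attack spawns a hand-attached arrow for Humans or sling rock otherwise, charges it by timer and launches on release, with camera zoom and cooldown.
; Older hitbox melee and teleport test logic is left unconnected.
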(event OnComponentBeginOverlap(CapsuleComponent)
  (params (OverlappedComponent :type Primitive%20Component%20Object%20Reference) (OtherActor :type Actor%20Object%20Reference) (OtherComp :type Primitive%20Component%20Object%20Reference) (OtherBodyIndex :type Integer) (bFromSweep :type Boolean) (SweepResult :type Hit%20Result%20Structure%20%28by%20ref%29))
  ;[1 1 1] Melee Swing
)

(event OnComponentBeginOverlap(SwingHitbox)
  (params (OverlappedComponent :type Primitive%20Component%20Object%20Reference) (OtherActor :type Actor%20Object%20Reference) (OtherComp :type Primitive%20Component%20Object%20Reference) (OtherBodyIndex :type Integer) (bFromSweep :type Boolean) (SweepResult :type Hit%20Result%20Structure%20%28by%20ref%29))
  ;[1 1 1] Melee Swing
)

(event Custom|AnimationTimerFunc
  ;[1 1 1] Melee Swing
  (bind _returnvalue (Utilities|Time|SetTimerbyEvent (delegate Custom|TimerTick) 0.1 true))
  (Variables|Default|SetTimer%20Handle _returnvalue))

(event Custom|ChargeShot
  (bind _spawnedarrow (Variables|Default|GetSpawnedArrow))
  ;[1 1 1] Timed Functions Used for charging and coolDown **FOR BOW ATTK*
  (bind _output_get (Variables|Default|SetCharge%20Amount (+ 0.08 (Variables|Default|GetCharge%20Amount))))
  (bind _asctfplayer_state (Utilities|Casting|CastToCTFPlayerState (Variables|Default|GetPlayerState)))
  (if (Utilities|Enum|Equal(Enum) (Variables|/Script/GAME259A.CTFPlayerState|GetteamID _asctfplayer_state) "Human")
    (bind _asbp_arrow_combat (Utilities|Casting|CastToBP_ArrowCOMBAT _spawnedarrow))
    (Variables|/Game/Game_BP/Weapons/BP_ArrowCOMBAT.BP_ArrowCOMBAT_C|SetInitSpeedCharge _asbp_arrow_combat (Variables|Default|GetCharge%20Amount))
    (else
      (bind _asbp_rock_combat (Utilities|Casting|CastToBP_RockCOMBAT _spawnedarrow))
      (Variables|/Game/Game_BP/Weapons/BP_RockCOMBAT.BP_RockCOMBAT_C|SetInitSpeedCharge _asbp_rock_combat (Variables|Default|GetCharge%20Amount))))
  (if (or (> _output_get 1.5) (not (Variables|Default|GetIs%20Drawing%20Bow%200)))
    (Utilities|Time|ClearTimerbyFunctionName 0 "ChargeShot")))

(event Custom|Server_StartRangeActors
  ;[1 1 1] Ranged Attack
  ;;[1 1 1] Changes Your Weapon For Everyone In The Game
  (Rendering|SetActorHiddenInGame (Variables|Default|GetMelee%20Weapon) true)
  (Rendering|SetActorHiddenInGame (Variables|Default|GetBow) false)
  (bind _asctfplayer_state (Utilities|Casting|CastToCTFPlayerState (Variables|Default|GetPlayerState)))
  (if (Utilities|Enum|Equal(Enum) (Variables|/Script/GAME259A.CTFPlayerState|GetteamID _asctfplayer_state) "Alien")
    (Rendering|SetActorHiddenInGame (Variables|Default|GetSlingSpecialPiece) false)))

(event Custom|Server_EndRangeActors
  ;[1 1 1] Ranged Attack
  (Rendering|SetActorHiddenInGame (Variables|Default|GetBow) true)
  (bind _asctfplayer_state (Utilities|Casting|CastToCTFPlayerState (Variables|Default|GetPlayerState)))
  (if (Utilities|Enum|Equal(Enum) (Variables|/Script/GAME259A.CTFPlayerState|GetteamID _asctfplayer_state) "Alien")
    (Rendering|SetActorHiddenInGame (Variables|Default|GetSlingSpecialPiece) true))
  (Utilities|Time|SetTimerbyFunctionName 0 "LowerCoolDown" 0.2 true)
  (Rendering|SetActorHiddenInGame (Variables|Default|GetMelee%20Weapon) false))

(event Custom|Server
  (Variables|Default|SetAimPitch (.pitch (Transformation|GetWorldRotation (Variables|Default|GetThirdPersonCamera))))
  (CallFunction|MultiHelp))

(event Custom|AttackAnimMulti
  ;[1 1 1] TEST
  (Networking|SwitchHasAuthority
    (:Authority
      (CallFunction|ServerAttackTest)
      (Utilities|FlowControl|Delay 0.4)
      (Networking|SwitchHasAuthority
        (:Authority
          (Variables|Default|SetisAttacking false))))))

(event Custom|ClientSideAim
  (Utilities|Time|ClearTimerbyFunctionName 0 "ReturnCam")
  (Utilities|Time|SetTimerbyFunctionName 0 "AimCam" (Utilities|Time|GetWorldDeltaSeconds) true))

(event Custom|ClientSideReturnAim
  (Utilities|Time|ClearTimerbyFunctionName 0 "AimCam")
  (Utilities|Time|SetTimerbyFunctionName 0 "ReturnCam" (Utilities|Time|GetWorldDeltaSeconds) true))

(event Custom|Multicast_MeleeAttack
  ;[1 1 1] Melee Swing
  ;;[1 1 1] Lets Everyone Know We Are Attacking
  (Development|PrintString "left clicked")
  (if (not (Variables|Default|GetisAttacking))
    (Audio|PlaySoundatLocation "/Game/VFX_Folder/SFX/Sound_Punch_JMF.Sound_Punch_JMF" (Transformation|GetActorLocation (Game|Player|GetPlayerPawn 0)) "0, 0, 0" 1.0 1.0 0.0 0 0 0)
    (CallFunction|AnimationTimerFunc)
    (Variables|Default|SetisAttacking true)
    (Variables|Default|SetbIsSwinging true)
    (Utilities|FlowControl|Delay 1.0)
    (Variables|Default|SetbIsSwinging false)
    (Variables|Default|SetisAttacking false)))

(event Custom|MultiHelp
  (Networking|SwitchHasAuthority
    (:Authority
      (Utilities|FlowControl|Delay 0.4)
      (Networking|SwitchHasAuthority
        (:Authority
          (Variables|Default|SetAimPitch (.pitch (Transformation|GetWorldRotation (Variables|Default|GetThirdPersonCamera)))))))))

(event Custom|ServerAttackTest
  (bind _attackmeleelocation (Variables|Default|GetAttackMeleeLocation))
  (bind _returnvalue (Transformation|GetWorldLocation _attackmeleelocation))
  ;[1 1 1] TEST
  (bind (_outactors _returnvalue_2) (Collision|SphereOverlapActors _returnvalue 1e+02 (Utilities|Array|MakeArray "ObjectTypeQuery3") 0 (Utilities|Array|MakeArray self)))
  (Rendering|Debug|DrawDebugSphere _returnvalue 1e+02 12 "(R=1.000000,G=0.013544,B=0.000000,A=1.000000)" 1.0 1.0)
  (if _returnvalue_2
    (for _array_element _outactors
      (if (Actor|ActorHasTag _array_element "Player")
        (bind _asbase_character (Utilities|Casting|CastToBaseCharacter _array_element))
        (bind _asctfplayer_state (Utilities|Casting|CastToCTFPlayerState (Variables|/Script/Engine.Pawn|GetPlayerState _asbase_character)))
        (bind _asctfplayer_state_2 (Utilities|Casting|CastToCTFPlayerState (Variables|Default|GetPlayerState)))
        (if (Utilities|Enum|NotEqual(Enum) (Variables|/Script/GAME259A.CTFPlayerState|GetteamID _asctfplayer_state_2) (Variables|/Script/GAME259A.CTFPlayerState|GetteamID _asctfplayer_state))
          (Game|Damage|ApplyDamage _array_element 2e+01 (Pawn|GetController) self)
          (Development|PrintString "Deal Damage")
          (else
            (Development|PrintString "Same Team")))))))

(event Custom|ServerAttack
  ;[1 1 1] TEST
  (Variables|Default|SetisAttacking true)
  (Utilities|FlowControl|Delay 0.6)
  (CallFunction|AttackAnimMulti))

(event Custom|LowerCoolDown
  ;[1 1 1] Timed Functions Used for charging and coolDown **FOR BOW ATTK*
  (bind _output_get (Variables|Default|SetCool%20Down (Math|Float|Clamp(Float) (- (Variables|Default|GetCool%20Down) 0.1))))
  (if (<= _output_get 0.0)
    (Utilities|Time|ClearTimerbyFunctionName 0 "LowerCoolDown")))

(event Custom|ReturnCam
  (bind _returnvalue (Utilities|Time|GetWorldDeltaSeconds))
  (bind _cameraboom (Variables|Default|GetCameraBoom))
  (bind _output_get (Variables|/Script/Engine.SpringArmComponent|SetTargetArmLength _cameraboom (Math|Interpolation|FInterpTo (Variables|/Script/Engine.SpringArmComponent|GetTargetArmLength _cameraboom) 3e+02 _returnvalue 5.0)))
  (Variables|/Script/Engine.SpringArmComponent|SetSocketOffset _cameraboom (Math|Interpolation|VInterpTo (Variables|/Script/Engine.SpringArmComponent|GetSocketOffset _cameraboom) "0, 0, 0" _returnvalue 5.0))
  (if (== _output_get 3e+02)
    (Utilities|Time|ClearTimerbyFunctionName 0 "AimCam")))

(event Custom|ShootArrow
  (bind _spawnedarrow (Variables|Default|GetSpawnedArrow))
  ;[1 1 1] Ranged Attack
  ;;[1 1 1] Tell Ther Server To Shoot The Arrow
  (Utilities|Time|ClearTimerbyFunctionName 0 "AimCam")
  (Utilities|Time|SetTimerbyFunctionName 0 "ReturnCam" (Utilities|Time|GetWorldDeltaSeconds) true)
  (Transformation|DetachFromActor (Variables|Default|GetSpawnedArrow) "KeepWorld" "KeepWorld" "KeepWorld")
  (bind _asctfplayer_state (Utilities|Casting|CastToCTFPlayerState (Variables|Default|GetPlayerState)))
  (if (Utilities|Enum|Equal(Enum) (Variables|/Script/GAME259A.CTFPlayerState|GetteamID _asctfplayer_state) "Human")
    (bind _asbp_arrow_combat (Utilities|Casting|CastToBP_ArrowCOMBAT _spawnedarrow))
    (Default|BeginProjectile _asbp_arrow_combat (* (Variables|Default|GetCharge%20Amount) 1.5))
    (else
      (bind _asbp_rock_combat (Utilities|Casting|CastToBP_RockCOMBAT _spawnedarrow))
      (Default|BeginProjectile _asbp_rock_combat (* (Variables|Default|GetCharge%20Amount) 1.5))))
  (Variables|Default|SetCharge%20Amount 0.0))

(event Custom|AimCam
  (bind _returnvalue (Utilities|Time|GetWorldDeltaSeconds))
  (bind _cameraboom (Variables|Default|GetCameraBoom))
  (bind _output_get (Variables|/Script/Engine.SpringArmComponent|SetTargetArmLength _cameraboom (Math|Interpolation|FInterpTo (Variables|/Script/Engine.SpringArmComponent|GetTargetArmLength _cameraboom) 1.5e+02 _returnvalue 2.0)))
  (Variables|/Script/Engine.SpringArmComponent|SetSocketOffset _cameraboom (Math|Interpolation|VInterpTo (Variables|/Script/Engine.SpringArmComponent|GetSocketOffset _cameraboom) "0,60.000000,10.000000" _returnvalue 1.0))
  (if (== _output_get 1.5e+02)
    (Utilities|Time|ClearTimerbyFunctionName 0 "AimCam")))

(event Custom|TimerTick
  ;[1 1 1] Melee Swing
  (bind _output_get (Variables|Default|SetAnimation%20Timer (+ (Variables|Default|GetAnimation%20Timer) 0.1)))
  (if (> _output_get 0.8)
    (Utilities|Time|ClearandInvalidateTimerbyHandle (Variables|Default|GetTimer%20Handle))
    (Variables|Default|SetAnimation%20Timer 0.0)))

(event Custom|Server_StopRangeAttack
  ;[1 1 1] Ranged Attack
  (if (Variables|Default|GetIs%20Drawing%20Bow%200)
    (if (<= (Variables|Default|GetCool%20Down) 0.0)
      (Audio|PlaySoundatLocation "/Game/VFX_Folder/SFX/Sound_Bow_JMF.Sound_Bow_JMF" (Transformation|GetActorLocation (Game|Player|GetPlayerPawn 0)) "0, 0, 0" 1.0 1.0 0.0 0 0 0)
      (Variables|Default|SetCool%20Down 0.5)
      (CallFunction|ShootArrow)
      (Utilities|FlowControl|Delay 0.2)
      (Variables|Default|SetbUseControllerRotationYaw false)
      (Variables|Default|SetIs%20Drawing%20Bow%200 false)
      (Utilities|FlowControl|Delay 0.2)
      (CallFunction|ClientSideReturnAim)
      (CallFunction|ServerEndRangeActors))))

(event Custom|Server_StartRangeAttack
  ;[1 1 1] Ranged Attack
  ;;[1 1 1] Lets The Server Know we are Drawing Our Bow
  (if (not (Variables|Default|GetisAttacking))
    (if (<= (Variables|Default|GetCool%20Down) 0.0)
      (Variables|Default|SetbUseControllerRotationYaw true)
      (Variables|Default|SetIs%20Drawing%20Bow%200 true)
      (CallFunction|ServerStartRangeActors)
      (CallFunction|SpawnCorrespondingProjectile)
      (CallFunction|ClientSideAim))))

(event Collision|EventActorBeginOverlap
  (params (OtherActor :type Actor%20Object%20Reference)))

(event EventTick
  (params (DeltaSeconds :type Float%20%28single-precision%29))
  (if (Pawn|IsLocallyControlled)
    (CallFunction|Server)))

(event EventGetHit
  ;[1 1 1] Take Damage BP (NESSASARY TO REMOVE THE ALREADY HIT INVINCIBILITY)
)

(event Game|Damage|EventAnyDamage
  (params (Damage :type Float%20%28single-precision%29) (DamageType :type Damage%20Type%20Object%20Reference) (InstigatedBy :type Controller%20Object%20Reference) (DamageCauser :type Actor%20Object%20Reference))
  ;[1 1 1] TEST
  (Variables|Default|SetHealth (- (Variables|Default|GetHealth) Damage))
  (if (<= (Variables|Default|GetHealth) 0.0)
    (Class|BaseCharacter|Death)))

(event Input|ActionEvents|InputActionRangedAttack
  (params (Key :type Key%20Structure :default "None"))
  ;[1 1 1] Ranged Attack
  ;;[1 1 1] Tell Server We Want to Range Attack
  (:Pressed
    (bind _asctfplayer_state (Utilities|Casting|CastToCTFPlayerState (Variables|Default|GetPlayerState)))
    (Utilities|IsValid self
      (:Is%20Valid
        (if (not (Variables|/Script/GAME259A.CTFPlayerState|GetbIsSprinting _asctfplayer_state))
          (CallFunction|ServerStartRangeAttack)))
      (:Is%20Not%20Valid
        (Development|PrintString "not valid"))))
  (:Released
    (bind _asctfplayer_state_2 (Utilities|Casting|CastToCTFPlayerState (Variables|Default|GetPlayerState)))
    (Utilities|IsValid self
      (:Is%20Valid
        (if (not (Variables|/Script/GAME259A.CTFPlayerState|GetbIsSprinting _asctfplayer_state_2))
          (CallFunction|ServerStopRangeAttack)))
      (:Is%20Not%20Valid
        (Development|PrintString "not valid")))))

(event Input|ActionEvents|InputActionAbilityOne
  (params (Key :type Key%20Structure :default "None"))
  ;[1 1 1] This is for teleport ability. CPP version is really broke rn.
)

(event Input|ActionEvents|InputActionPauseMenu
  (params (Key :type Key%20Structure :default "None"))
  (bind _returnvalue (Game|GetPlayerController 0))
  ;[1 1 1] Pause Game
  (:Pressed
    (bind _returnvalue_2 (UserInterface|CreateWidget "/Game/UI/Menus/PauseMenu.PauseMenu_C"))
    (Variables|Default|SetPauseRefrence _returnvalue_2)
    (Variables|/Script/Engine.PlayerController|SetbShowMouseCursor _returnvalue true)
    (Input|DisableInput (Game|GetPlayerCharacter 0) _returnvalue)
    (UserInterface|Viewport|AddtoViewport (Variables|Default|GetPauseRefrence) 0)))

(event Input|MouseEvents|LeftMouseButton
  (params (Key :type Key%20Structure :default "None")))

(event Input|MouseEvents|LeftMouseButton
  (params (Key :type Key%20Structure :default "None"))
  ;[1 1 1] TEST
  (:Pressed
    (if (and (not (Variables|Default|GetisAttacking)) (not (Variables|Default|GetIs%20Drawing%20Bow%200)))
      (CallFunction|ServerAttack))))

(fn ConstructionScript)

(fn SpawnCorrespondingProjectile
  (bind _asctfplayer_state (Utilities|Casting|CastToCTFPlayerState (Variables|Default|GetPlayerState)))
  (if (Utilities|Enum|Equal(Enum) (Variables|/Script/GAME259A.CTFPlayerState|GetteamID _asctfplayer_state) "Human")
    (bind _returnvalue (Game|SpawnActorfromClass "/Game/Game_BP/Weapons/BP_ArrowCOMBAT.BP_ArrowCOMBAT_C" (Transformation|GetActorTransform) "Undefined" self 0))
    (bind _output_get (Variables|Default|SetSpawnedArrow _returnvalue))
    (Transformation|AttachComponentToComponent _output_get (Variables|Character|GetMesh) "RightHand" "SnapToTarget" "SnapToTarget" "SnapToTarget" false)
    (Transformation|AddActorLocalOffset (Variables|Default|GetSpawnedArrow) "-90.000000,5.500000,0.000000" false true)
    (Transformation|AddActorLocalRotation (Variables|Default|GetSpawnedArrow) "180.000000,-5.000000,0.000000" false false)
    (Utilities|Time|SetTimerbyFunctionName 0 "ChargeShot" 0.1 true)
    (else
      (bind _returnvalue_2 (Game|SpawnActorfromClass "/Game/Game_BP/Weapons/BP_RockCOMBAT.BP_RockCOMBAT_C" (Transformation|GetActorTransform) "Undefined" self 0))
      (bind _output_get_2 (Variables|Default|SetSpawnedArrow _returnvalue_2))
      (Transformation|AttachComponentToComponent _output_get_2 (Variables|Character|GetMesh) "RightHandSocketSling" "SnapToTarget" "SnapToTarget" "SnapToTarget" false)
      (Transformation|AddActorLocalOffset (Variables|Default|GetSpawnedArrow) "0, 0, 0" false true)
      (Transformation|AddActorLocalRotation (Variables|Default|GetSpawnedArrow) "0.000000,-90.000000,0.000000" false false)
      (Utilities|Time|SetTimerbyFunctionName 0 "ChargeShot" 0.1 true)))
  (return))