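; Test teleport ability projectile actor that moves the player character to where it hits.
; On BeginPlay it copies its Velocity variable into the ProjectileMovement component.
; On Hit it teleports player 0's character without sweep to the impact point, pushed out along the surface normal, then destroys itself.
; The construction script shrinks the Sphere component to half scale.
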(event EventBeginPlay
  (Variables|/Script/Engine.MovementComponent|SetVelocity (Variables|Default|GetProjectileMovement) (Variables|Default|GetVelocity)))

(event Collision|EventHit
  (params (MyComp :type Primitive%20Component%20Object%20Reference) (Other :type Actor%20Object%20Reference) (OtherComp :type Primitive%20Component%20Object%20Reference) (bSelfMoved :type Boolean) (HitLocation :type Vector :default "0, 0, 0") (HitNormal :type Vector :default "0, 0, 0") (NormalImpulse :type Vector :default "0, 0, 0") (Hit :type Hit%20Result%20Structure%20%28by%20ref%29))
  (if true
    (Transformation|SetActorLocation (Game|GetPlayerCharacter 0) (+ HitLocation (* HitNormal 1.2e+02)) false true)
    (Actor|DestroyActor)))

(fn ConstructionScript
  (Transformation|SetWorldScale3D (Variables|Default|GetSphere) "0.500000,0.500000,0.500000"))